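; BP_Database is an actor that holds the active database record and rule record and persists them through an ActorPersistence component.
; On BeginPlay it binds to the data-loaded signal, first generating a unique ID and marking itself dirty if none is valid.
; DataLoaded feeds the active records into DBUpdate, the client update event that stores both records and flags persistence dirty.
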(event Custom|DataLoaded
  ;[1 1 1] Data loaded from Database
  (CallFunction|DBUpdate (Variables|Default|GetActiveDBRecord) (Variables|Default|GetActiveDBRuleRecord)))

(event Custom|DBUpdate
  (params (DBRecord :type S%20DB%20Structure) (DBRecordRules :type S%20DB%20Rules%20Structure))
  ;[1 1 1] Client Database updates
  (Variables|Default|SetActiveDBRecord DBRecord)
  (Variables|Default|SetActiveDBRuleRecord DBRecordRules)
  (Class|PersistenceComponent|SetDirty (Variables|Default|GetActorPersistence) true))

(event EventBeginPlay
  (bind _actorpersistence (Variables|Default|GetActorPersistence))
  ;[1 1 1] Initial DB Setup
  (if (Class|DreamworldBlueprints|IsValidID (Class|PersistenceComponent|GetUniqueID (Variables|Default|GetActorPersistence)))
    (EventDispatchers|BindEventtoOnSignalDataLoaded (Variables|Default|GetActorPersistence) (delegate Custom|DataLoaded))
    (else
      (bind _returnvalue (Class|UniqueID|GenerateUniqueID))
      (Class|DreamworldBlueprints|SetUniqueID self _returnvalue)
      (Class|PersistenceComponent|SetDirty _actorpersistence true)
      (EventDispatchers|BindEventtoOnSignalDataLoaded _actorpersistence (delegate Custom|DataLoaded)))))

(fn ConstructionScript)